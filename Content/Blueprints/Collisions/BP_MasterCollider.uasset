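; BP_MasterCollider is a reusable trigger volume that drives level progression, checkpoints and death for BP_Player.
; When BP_Player begins overlapping its Box, it switches on ColliderType to pick the action.
; Level start triggers fire only if CurrentLevel matches, while death, level end and checkpoint act directly, with checkpoints passing the Arrow's world transform as the respawn point.
; The End type currently only prints a teleport debug message.
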(event OnComponentBeginOverlap(Box)
  (params (OverlappedComponent :type Primitive%20Component%20Object%20Reference) (OtherActor :type Actor%20Object%20Reference) (OtherComp :type Primitive%20Component%20Object%20Reference) (OtherBodyIndex :type Integer) (bFromSweep :type Boolean) (SweepResult :type Hit%20Result%20Structure%20%28by%20ref%29))
  (bind _asbp_player (Utilities|Casting|CastToBP_Player OtherActor))
  (switch Utilities|FlowControl|Switch|SwitchonE_CollidersType (Variables|Default|GetColliderType)
    (:NewEnumerator0
      (if (Utilities|Enum|Equal(Enum) (Variables|/Game/Blueprints/BP_Player.BP_Player_C|GetCurrentLevel _asbp_player) "NewEnumerator0")
        (Default|StartLevel1 _asbp_player)))
    (:NewEnumerator1
      (if (Utilities|Enum|Equal(Enum) (Variables|/Game/Blueprints/BP_Player.BP_Player_C|GetCurrentLevel _asbp_player) "NewEnumerator1")
        (Default|StartLevel2 _asbp_player)))
    (:NewEnumerator2
      (if (Utilities|Enum|Equal(Enum) (Variables|/Game/Blueprints/BP_Player.BP_Player_C|GetCurrentLevel _asbp_player) "NewEnumerator2")
        (Development|PrintString "TP TO ENDING LEVEL")))
    (:NewEnumerator3
      (Default|Die _asbp_player))
    (:NewEnumerator4
      (Development|PrintString "SET CHECKPOINT")
      (Default|NewCheckpoint _asbp_player (Transformation|GetWorldTransform (Variables|Default|GetArrow))))
    (:NewEnumerator5
      (Default|EndLevel1 _asbp_player))
    (:NewEnumerator6
      (Default|EndLevel2 _asbp_player))))

(fn ConstructionScript)